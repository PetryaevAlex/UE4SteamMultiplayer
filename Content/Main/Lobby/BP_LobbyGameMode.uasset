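; Lobby game mode that manages connected players, host map settings, character selection, kicking and match launch for a multiplayer session.
; It tracks joining and leaving controllers, pushing settings, player info and character availability to each through controller reference messages.
; Character changes claim a free slot, then respawn and possess a pawn at the last PlayerStart.
; Launch shows loading screens, then server-travels to the level matching the selected map ID.
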(event Custom|SpawnPlayer
  (params (PlayerController :type Player%20Controller%20Object%20Reference)))

(event Custom|StartLoadingScreen
  ;[1 1 1] Show the Loading Screen and Launches selected Level
  (for _array_element (Variables|Default|GetConnectedPlayers)
    (bind _playercontroller (Class|BPILobbyPC|LobbyPCRef(Message) _array_element))
    (Default|ShowLoadingScreen _playercontroller))
  (CallFunction|LaunchGame))

(event Custom|HostUpdateGameSettings
  (params (SelectedMapImage :type Texture%202D%20Object%20Reference) (SelectedMapName :type Text) (SelectedMapTime :type Text) (SelectedMapID :type Integer))
  ;[1 1 1] Server Has Made Changes Say To Clients
  (Variables|Default|SetSelectedMapImage SelectedMapImage)
  (Variables|Default|SetSelectedMapName SelectedMapName)
  (Variables|Default|SetSelectedMapTime SelectedMapTime)
  (Variables|Default|SetSelectedMapID SelectedMapID)
  (for _array_element (Variables|Default|GetConnectedPlayers)
    (bind _playercontroller (Class|BPILobbyPC|LobbyPCRef(Message) _array_element))
    (Default|UpdateLobbySettings _playercontroller (Variables|Default|GetSelectedMapImage) (Variables|Default|GetSelectedMapName) (Variables|Default|GetSelectedMapTime))))

(event Custom|PlayerKicked
  (params (PlayerID :type Integer))
  ;[1 1 1] Kick Selected Player From Game Session
  (bind _playercontroller (Class|BPILobbyPC|LobbyPCRef(Message) (Utilities|Array|Get(acopy) (Variables|Default|GetConnectedPlayers) PlayerID)))
  (Default|Kicked _playercontroller))

(event Custom|EveryoneUpdate
  ;[1 1 1] Updates All Connected Players
  (bind _output_get (Variables|Default|SetCurrentPlayers (Utilities|Array|Length (Variables|Default|GetConnectedPlayers))))
  (if (> _output_get 0)
    (Utilities|Array|Clear (Variables|Default|GetConnectedPlayersInfo))
    (for _array_element (Variables|Default|GetConnectedPlayers)
      (bind _playercontroller (Class|BPILobbyPC|LobbyPCRef(Message) _array_element))
      (Utilities|Array|AddUnique (Variables|Default|GetConnectedPlayersInfo) (Variables|/Game/Main/Lobby/BP_LobbyPC.BP_LobbyPC_C|GetPlayerSettings _playercontroller))
      (Default|UpdateNumberOfPlayers _playercontroller (Variables|Default|GetCurrentPlayers) (Variables|Default|GetMaxPlayers)))
    (for _array_element_2 (Variables|Default|GetConnectedPlayers)
      (bind _playercontroller_2 (Class|BPILobbyPC|LobbyPCRef(Message) _array_element_2))
      (Default|AddPlayerInfo _playercontroller_2 (Variables|Default|GetConnectedPlayersInfo))
      (Default|UpdateAvailableCharacters _playercontroller_2 (Variables|Default|GetAvailablePlayers))
      (CallFunction|AddtoKickList))
    (bind _array_element_3 (Utilities|Array|ForEachLoopwithBreak (Variables|Default|GetConnectedPlayersInfo))
      (:LoopBody
        (if (== (.PlayerCharacter (Utilities|Struct|BreakS_PlayerInfo _array_element_3)) 0)
          (Variables|Default|SetCanWeStart false)
          (CallFunction|CannotStartGame)
          (else
            (Variables|Default|SetCanWeStart true)))))))

(event Custom|AddToKickList
  ;[1 1 1] Add Connected Players To Kick List
  (bind _playercontroller (Class|BPILobbyPC|LobbyPCRef(Message) (Variables|Default|GetConnectedPlayer)))
  (Default|AddPlayertoKickWindow _playercontroller))

(event Custom|CannotStartGame
  ;[1 1 1] Updates All Connected Players
  (Utilities|Array|ForEachLoopwithBreak (Variables|Default|GetConnectedPlayersInfo)) ; enters at Break
)

(event Custom|LaunchGame
  (bind _returnvalue (Game|GetPlayerController 0))
  ;[1 1 1] Show the Loading Screen and Launches selected Level
  (switch int (Variables|Default|GetSelectedMapID)
    (:0
      (Development|ExecuteConsoleCommand "servertravel /Game/Maps/Level1" _returnvalue))
    (:1
      (Development|ExecuteConsoleCommand "servertravel /Game/Maps/Level2" _returnvalue))))

(event Custom|ChangeCharacter
  (params (ConnectedPlayer :type Player%20Controller%20Object%20Reference) (CharacterClass :type Character%20Class%20Reference) (ChangeStatus :type Boolean))
  (bind _returnvalue (Pawn|GetControlledPawn ConnectedPlayer))
  (bind _spawnpoints (Variables|Default|GetSpawnPoints))
  ;[1 1 1] Spawns The Selected Character Wich Player Choose
  (if (not ChangeStatus)
    (Utilities|IsValid _returnvalue
      (:Is%20Valid
        (Actor|DestroyActor _returnvalue))
      (:Is%20Not%20Valid
        _))
    (bind _returnvalue_2 (Game|SpawnActorfromClass CharacterClass (Transformation|GetActorTransform (Utilities|Array|Get(acopy) _spawnpoints (- (Utilities|Array|Length _spawnpoints) 1))) "AlwaysSpawn" 0 0))
    (Pawn|Possess ConnectedPlayer _returnvalue_2)))

(event EventOnLogout
  (params (ExitingController :type Controller%20Object%20Reference))
  (bind _connectedplayers (Variables|Default|GetConnectedPlayers))
  ;[1 1 1] Remove The Connected Player Information and get their character available and then update everyone
  (bind (_array_element _array_index) (Utilities|Array|ForEachLoopwithBreak _connectedplayers :!label _label)
    (:LoopBody
      (if (== _array_element ExitingController)
        (goto _label Break)))
    (:Completed
      (bind _playercontroller (Class|BPILobbyPC|LobbyPCRef(Message) (Utilities|Array|Get(acopy) _connectedplayers _array_index)))
      (Utilities|Array|SetArrayElem (Variables|Default|GetAvailablePlayers) (Variables|/Game/Main/Lobby/BP_LobbyPC.BP_LobbyPC_C|GetSelectedCharacter _playercontroller) false)
      (Utilities|Array|RemoveIndex (Variables|Default|GetConnectedPlayers) _array_index)
      (Utilities|Array|RemoveIndex (Variables|Default|GetConnectedPlayersInfo) _array_index)
      (CallFunction|EveryoneUpdate))))

(event EventBeginPlay
  ;[1 1 1] Begin play
  (bind _outactors (Actor|GetAllActorsOfClass "/Script/Engine.PlayerStart"))
  (Variables|Default|SetSpawnPoints _outactors)
  (bind _game_instance (Class|BPIGameInstance|SteamGameInstanceRef(Message) (Game|GetGameInstance)))
  (Variables|Default|SetServerName (Variables|/Game/Main/BP_SteamGameInstance.BP_SteamGameInstance_C|GetServerName _game_instance))
  (Variables|Default|SetMaxPlayers (Variables|/Game/Main/BP_SteamGameInstance.BP_SteamGameInstance_C|GetMaxPlayers _game_instance)))

(event EventPostLogin
  (params (NewPlayer :type Player%20Controller%20Object%20Reference))
  ;[1 1 1] Initial Setup Run When New Client Connects To Session
  (bind _output_get (Variables|Default|SetConnectedPlayer NewPlayer))
  (Utilities|Array|AddUnique (Variables|Default|GetConnectedPlayers) _output_get)
  (Utilities|FlowControl|Delay 1.0)
  (bind _playercontroller (Class|BPILobbyPC|LobbyPCRef(Message) (Variables|Default|GetConnectedPlayer)))
  (Default|InitialSetup _playercontroller (Variables|Default|GetServerName) (Variables|Default|GetSelectedMapImage) (Variables|Default|GetSelectedMapName) (Variables|Default|GetSelectedMapTime))
  (CallFunction|SpawnPlayer (Variables|Default|GetConnectedPlayer)))

(fn ConstructionScript)

(fn GetCharacters
  (params (SelectedCharacterID :type Integer) (PreviousSelection :type Integer))
  (if (not (Math|Boolean|Equal(Boolean) (Utilities|Array|Get(acopy) (Variables|Default|GetAvailablePlayers) SelectedCharacterID) true))
    (Utilities|Array|SetArrayElem (Variables|Default|GetAvailablePlayers) SelectedCharacterID true)
    (Utilities|Array|SetArrayElem (Variables|Default|GetAvailablePlayers) PreviousSelection false)
    (return (Utilities|Array|Get(acopy) (Variables|Default|GetCharacters) SelectedCharacterID))))

(fn LobbyGameModeRef
  (return self))