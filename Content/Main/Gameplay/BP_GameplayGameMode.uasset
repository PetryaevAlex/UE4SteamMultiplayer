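; Gameplay game mode for a Steam session-based multiplayer game, handling player spawning, chat and logout.
; SpawnPlayer destroys a controller's existing pawn or, only if none exists, spawns and possesses the selected character at a random PlayerStart.
; Controllers gathered in OnSwapPlayerControllers receive chat updates.
; On logout it asks the Steam game instance, via interface message, to destroy the leaving player's session so they can join new games.
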(event Custom|SpawnPlayer
  (params (PlayerController :type Player%20Controller%20Object%20Reference) (SelectedCharacter :type Character%20Class%20Reference))
  (bind _returnvalue (Pawn|GetControlledPawn PlayerController))
  ;[1 1 1] Spawn Player At Random player start location
  (Development|PrintString "Spawn Player" true true "(R=0.000000,G=0.660000,B=1.000000,A=1.000000)" 2e+01)
  (bind _outactors (Actor|GetAllActorsOfClass "/Script/Engine.PlayerStart"))
  (Variables|Default|SetSpawnPoints _outactors)
  (Utilities|IsValid _returnvalue
    (:Is%20Valid
      (Actor|DestroyActor _returnvalue))
    (:Is%20Not%20Valid
      (bind _returnvalue_2 (Game|SpawnActorfromClass SelectedCharacter (Transformation|GetActorTransform (Utilities|Array|Get(acopy) (Variables|Default|GetSpawnPoints) (Math|Random|RandomIntegerinRange 0 (- (Utilities|Array|Length (Variables|Default|GetSpawnPoints)) 1)))) "Undefined" 0 0))
      (Pawn|Possess PlayerController _returnvalue_2))))

(event Custom|UpdateChat
  (params (Sender :type Text) (ChatText :type Text))
  ;[1 1 1] Update chat for all clients
  (for _array_element (Variables|Default|GetAllPlayerControllers)
    (bind _playercontroller (Class|BPIGameplayPC|GameplayPCRef(Message) _array_element))
    (Default|UpdateChatWindow _playercontroller Sender ChatText)))

(event EventOnSwapPlayerControllers
  (params (OldPC :type Player%20Controller%20Object%20Reference) (NewPC :type Player%20Controller%20Object%20Reference))
  (Utilities|Array|Add (Variables|Default|GetAllPlayerControllers) NewPC))

(event EventOnLogout
  (params (ExitingController :type Controller%20Object%20Reference))
  ;[1 1 1] On logout and destroy connected player's session so they can join new games
  (bind _playercontroller (Class|BPIGameplayPC|GameplayPCRef(Message) ExitingController))
  (bind _game_instance (Class|BPIGameInstance|SteamGameInstanceRef(Message) (Game|GetGameInstance)))
  (Class|BPIGameInstance|DestroySessionCaller(Message) _game_instance _playercontroller))

(fn ConstructionScript)

(fn GameplayGameModeRef
  (return self))